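; Enemy character base that repeatedly attacks with a child-actor weapon and reacts to damage.
; From BeginPlay it loops: wait a second, play a random attack montage, wait out its duration, with no alive check.
; Damage lowers health in BPACStats, turns the enemy toward the damage causer, then plays a hit react or triggers death.
; Both outcomes switch off weapon damage; death also disables further damage, stops montages and calls OnDeath.
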(event EventTick
  (params (DeltaSeconds :type Float%20%28single-precision%29)))

(event EventBeginPlay
  (Utilities|FlowControl|Delay 1.0 :!label _label)
  (bind _duration (CallFunction|Attack))
  (Utilities|FlowControl|Delay _duration)
  (goto _label))

(event Game|Damage|EventAnyDamage
  (params (Damage :type Float%20%28single-precision%29) (DamageType :type Damage%20Type%20Object%20Reference) (InstigatedBy :type Controller%20Object%20Reference) (DamageCauser :type Actor%20Object%20Reference))
  (CallFunction|OnTakeDamage Damage DamageCauser))

(fn ConstructionScript
  (Actor|SetOwner (Variables|/Script/Engine.ChildActorComponent|GetChildActor (Variables|Default|GetWeaponActor)) self))

(fn OnTakeDamage
  (params (Amount :type Float%20%28double-precision%29) (DamageCauser :type Actor%20Object%20Reference))
  (Default|DamageHealth (Variables|Default|GetBP_AC_Stats) Amount)
  (Transformation|SetActorRotation (Math|Rotator|MakeRotator 0.0 0.0 (.yaw (Math|Rotator|FindLookatRotation (Transformation|GetActorLocation) (Transformation|GetActorLocation DamageCauser)))))
  (if (CallFunction|IsAlive)
    (CallFunction|PlayHitReact)
    (else
      (CallFunction|Death))))

(fn Death
  (bind _mesh (Variables|Character|GetMesh))
  (bind _returnvalue (Components|SkeletalMesh|GetAnimInstance _mesh))
  (Variables|Actor|SetbCanBeDamaged false)
  (CallFunction|DeactivateDamage)
  (Animation|Montage|MontageStop _returnvalue 0.0 (Animation|Montage|GetCurrentActiveMontage _returnvalue))
  (Default|CallOnDeath))

(fn IsAlive
  (return (> (Variables|/Game/MyContent/Core/BP_AC_Stats.BP_AC_Stats_C|GetHealth (Variables|Default|GetBP_AC_Stats)) 0.0)))

(fn Attack
  (if (Utilities|Array|IsNotEmpty (Variables|Default|GetAttackAnims))
    (bind _returnvalue (Animation|Montage|MontagePlay (Components|SkeletalMesh|GetAnimInstance (Variables|Character|GetMesh)) (.OutItem (Utilities|Array|Random (Variables|Default|GetAttackAnims))) 1.0 "Duration" 0.0 true))
    (return _returnvalue)))

(fn ActivateDamage
  (bind _asbp_weapon (Utilities|Casting|CastToBP_Weapon (Variables|/Script/Engine.ChildActorComponent|GetChildActor (Variables|Default|GetWeaponActor))))
  (Default|ActivateDamage _asbp_weapon))

(fn DeactivateDamage
  (bind _asbp_weapon (Utilities|Casting|CastToBP_Weapon (Variables|/Script/Engine.ChildActorComponent|GetChildActor (Variables|Default|GetWeaponActor))))
  (Default|DeactivateDamage _asbp_weapon))

(fn PlayHitReact
  (Animation|PlayAnimMontage (Variables|Default|GetHitReactAnim) 1.0 "None")
  (CallFunction|DeactivateDamage))
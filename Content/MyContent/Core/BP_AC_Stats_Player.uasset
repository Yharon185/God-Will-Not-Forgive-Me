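; Player stats component that tracks XP, levelling and stamina, firing event dispatchers when they change.
; AddXP triggers one LevelUp upon reaching MaxXP, carrying the surplus over.
; A looping Delay from BeginPlay regenerates stamina until full, while Tick prints it for debugging through a Delay.
; StaminaCheck tests for the fixed cost that StaminaUsage deducts; regen and usage write Stamina directly, bypassing the clamped setter.
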(event EventBeginPlay
  (CallFunction|StaminaRegen 0.2 :!label _label)
  (Utilities|FlowControl|Delay 0.01)
  (goto _label))

(event EventTick
  (params (DeltaSeconds :type Float%20%28single-precision%29))
  (Utilities|FlowControl|Delay 1.0)
  (Development|PrintString (Utilities|String|ToString(Float) (Variables|Default|GetStamina))))

(fn SetXP
  (params (XP :type Float%20%28double-precision%29))
  (Variables|Default|SetXP (Math|Float|Max(Float) XP 0.0))
  (Default|CallOnXPChanged))

(fn SetMaxXP
  (params (MaxXP :type Float%20%28double-precision%29))
  (Variables|Default|SetMaxXP (Math|Float|Max(Float) MaxXP 0.0))
  (Default|CallOnXPChanged))

(fn AddXP
  (params (Amount :type Float%20%28double-precision%29))
  (CallFunction|SetXP (+ (Variables|Default|GetXP) Amount))
  (Default|CallOnXPAdded Amount)
  (if (>= (Variables|Default|GetXP) (Variables|Default|GetMaxXP))
    (CallFunction|LevelUp)))

(fn LevelUp
  (CallFunction|SetLevel (+ (Variables|Default|GetLevel) 1.0))
  (CallFunction|SetXP (- (Variables|Default|GetXP) (Variables|Default|GetMaxXP)))
  (Default|CallOnLevelUp))

(fn SetStamina
  (params (Stamina :type Float%20%28double-precision%29))
  (Variables|Default|SetStamina (Math|Float|Clamp(Float) Stamina 0.0 (Variables|Default|GetMaxStamina)))
  (Default|CallOnStaminaChange))

(fn SetMaxStamina
  (params (MaxStamina :type Float%20%28double-precision%29))
  (Variables|Default|SetMaxStamina (Math|Float|Max(Float) MaxStamina 0.0))
  (Default|CallOnStaminaChange))

(fn StaminaRegen
  (params (RegenAmount :type Float%20%28double-precision%29))
  (if (not (>= (Variables|Default|GetStamina) (Variables|Default|GetMaxStamina)))
    (Variables|Default|SetStamina (+ (Variables|Default|GetStamina) RegenAmount))
    (Default|CallOnStaminaChange)))

(fn StaminaUsage
  (Variables|Default|SetStamina (- (Variables|Default|GetStamina) 2e+01))
  (Default|CallOnStaminaChange))

(fn StaminaCheck
  (if (>= (Variables|Default|GetStamina) 2e+01)
    (Variables|Default|SetStaminaCheckBool true)
    (if (Variables|Default|GetStaminaCheckBool)
      (return true))
    (else
      (Variables|Default|SetStaminaCheckBool false))))
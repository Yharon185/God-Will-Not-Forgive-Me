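; Player character for melee combat, with camera-relative movement, directional jump montages, and health damage with hit reactions.
; Stamina-gated combo attacks step through a montage array, with functions to reopen or reset the combo and toggle child-actor weapon damage.
; Soft targeting filters living, unobstructed actors by control-yaw angle; the closest-target pick effectively returns the first, as its distance check never passes.
; Motion warping aims attacks at that target, otherwise a timeline turns toward control yaw.
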(event Custom|LerpActorToControlRotation
  (params (Duration :type Float%20%28double-precision%29))
  (Components|Timeline|SetPlayRate (Variables|Default|GetTL_LerpActorToControlRotation) (/ 1.0 (Math|Float|Max(Float) Duration 0.0001)))
  (Variables|Default|SetStartLerpRotation (Transformation|GetActorRotation))
  (bind _alpha (Timeline|TL_LerpActorToControlRotation PlayFromStart)
    (:Update
      (Transformation|SetActorRotation (Math|Rotator|Lerp(Rotator) (Variables|Default|GetStartLerpRotation) (Math|Rotator|MakeRotator 0.0 0.0 (.yaw (Pawn|GetControlRotation :!class /Script/Engine.Pawn))) _alpha true)))))

(event EventOnJumped
  (CallFunction|PlayDirectionalJumpAnim))

(event EventOnLanded
  (params (Hit :type Hit%20Result%20Structure%20%28by%20ref%29))
  (Animation|PlayAnimMontage (Variables|Default|GetLandAnim) 1.0 "None"))

(event Game|Damage|EventAnyDamage
  (params (Damage :type Float%20%28single-precision%29) (DamageType :type Damage%20Type%20Object%20Reference) (InstigatedBy :type Controller%20Object%20Reference) (DamageCauser :type Actor%20Object%20Reference))
  (Default|DamageHealth (Variables|Default|GetBP_AC_Stats) Damage)
  (Transformation|SetActorRotation (Math|Rotator|MakeRotator 0.0 0.0 (.yaw (Math|Rotator|FindLookatRotation (Transformation|GetActorLocation) (Transformation|GetActorLocation DamageCauser)))))
  (CallFunction|PlayHitReact))

(event EventBeginPlay)

(fn ConstructionScript
  (CallFunction|InitialiseWeapon))

(fn ControlCamera
  (params (Axis :type Vector%202D%20Structure))
  (Utilities|FlowControl|Sequence
    (:then_0
      (Pawn|Input|AddControllerYawInput (.x Axis)))
    (:then_1
      (Pawn|Input|AddControllerPitchInput (.y Axis)))))

(fn MoveCharacter
  (params (Axis :type Vector%202D%20Structure))
  (bind _returnvalue (Pawn|GetControlRotation :!class /Script/Engine.Pawn))
  (bind (_x _y) (Math|Vector2D|BreakVector2D Axis))
  (bind _returnvalue_2 (Math|Rotator|MakeRotator 0.0 0.0 (.yaw _returnvalue)))
  (Utilities|FlowControl|Sequence
    (:then_0
      (Pawn|Input|AddMovementInput (Math|Vector|GetRightVector _returnvalue_2) _x false))
    (:then_1
      (Pawn|Input|AddMovementInput (Math|Vector|GetForwardVector _returnvalue_2) _y false))
    (:then_2
      (Variables|/Script/Engine.CharacterMovementComponent|SetbOrientRotationToMovement (Variables|Character|GetCharacterMovement) (<= (Class|KismetMathLibrary|VSize2DSquared Axis) 0.0)))))

(fn TryJump
  (params (Pressed/Released :type Boolean))
  (if (Variables|Default|GetIsNextComboAllowed)
    (if Pressed/Released
      (Character|Jump)
      (else
        (Character|StopJumping)))))

(fn PlayDirectionalJumpAnim
  (if (or (CallFunction|IsAcotrDirectionBetween -45.0 45.0) (<= (Math|Vector|VectorLengthXY (Transformation|GetVelocity)) 0.0))
    (Animation|PlayAnimMontage (Variables|Default|GetJumpForwardAnim) 1.0 "None")
    (elif (CallFunction|IsAcotrDirectionBetween 45.0 125.0)
      (Animation|PlayAnimMontage (Variables|Default|GetJumpRightAnim) 1.0 "None")
      (elif (CallFunction|IsAcotrDirectionBetween -125.0 -45.0)
        (Animation|PlayAnimMontage (Variables|Default|GetJumpLeftAnim) 1.0 "None")
        (else
          (Animation|PlayAnimMontage (Variables|Default|GetJumpBackAnim) 1.0 "None"))))))

(fn GetActorDirection
  (return (Class|KismetAnimationLibrary|CalculateDirection (Transformation|GetVelocity) (Transformation|GetActorRotation))))

(fn IsAcotrDirectionBetween
  (params (Minimum :type Float%20%28double-precision%29) (Maximum :type Float%20%28double-precision%29))
  (bind _returnvalue (CallFunction|GetActorDirection))
  (return (and (>= _returnvalue Minimum) (<= _returnvalue Maximum))))

(fn BasicComboAttack
  (bind _stamcheck (Default|StaminaCheck (Variables|Default|GetStats%20Component%20%28Player%29)))
  (if _stamcheck
    (if (and (Variables|Default|GetIsNextComboAllowed) (not (AI|Components|NavMovement|IsFalling (Variables|Character|GetCharacterMovement))))
      (Variables|Default|SetIsNextComboAllowed false)
      (Default|StaminaUsage (Variables|Default|GetStats%20Component%20%28Player%29))
      (bind _actor (CallFunction|FindAttackTargets))
      (bind _output_get (LocalVariables|SetLTestTarget _actor))
      (CallFunction|SetWarpTarget _output_get)
      (CallFunction|PlayReleventComboAnim)
      (CallFunction|IncrementComboCounter)
      (if (not (Utilities|IsValid (LocalVariables|GetLTestTarget)))
        (CallFunction|LerpActortoControlRotation 0.2)))))

(fn PlayReleventComboAnim
  (if (Utilities|Array|IsValidIndex (Variables|Default|GetBasicAttackComboAnims) (Variables|Default|GetCombo))
    (Animation|Montage|MontagePlay (Components|SkeletalMesh|GetAnimInstance (Variables|Character|GetMesh)) (Utilities|Array|Get(acopy) (Variables|Default|GetBasicAttackComboAnims) (Variables|Default|GetCombo)) 1.0 "MontageLength" 0.0 true)))

(fn IncrementComboCounter
  (bind _result (Math|Integer|IncrementInt (Variables|Default|GetCombo))
    (:%20%20
      (if (not (Utilities|Array|IsValidIndex (Variables|Default|GetBasicAttackComboAnims) _result))
        (Variables|Default|SetCombo 0)))))

(fn AllowNextCombo
  (Variables|Default|SetIsNextComboAllowed true))

(fn ResetCombo
  (Variables|Default|SetCombo 0))

(fn CancelAnim
  (CallFunction|AllowNextCombo)
  (CallFunction|ResetCombo))

(fn InitialiseWeapon
  (bind _asbp_weapon (Utilities|Casting|CastToBP_Weapon (Variables|/Script/Engine.ChildActorComponent|GetChildActor (Variables|Default|GetWeapon))))
  (Actor|SetOwner _asbp_weapon self))

(fn ActivateWeaponDamage
  (bind _asbp_weapon (Utilities|Casting|CastToBP_Weapon (Variables|/Script/Engine.ChildActorComponent|GetChildActor (Variables|Default|GetWeapon))))
  (Default|ActivateDamage _asbp_weapon))

(fn DeactivateWeaponDamage
  (bind _asbp_weapon (Utilities|Casting|CastToBP_Weapon (Variables|/Script/Engine.ChildActorComponent|GetChildActor (Variables|Default|GetWeapon))))
  (Default|DeactivateDamage _asbp_weapon))

(fn FindAttackTargets
  (Rendering|Debug|FlushPersistentDebugLines)
  (bind (_potentialtargets _bsuccess) (CallFunction|DetectPotentialTargets false))
  (if _bsuccess
    (bind (_targetswithinangle _success) (CallFunction|CompareTargetAngle _potentialtargets false))
    (if _success
      (bind _lclosestactor (CallFunction|FindTargetClosesttoSelf _targetswithinangle false))
      (return _lclosestactor)
      (else
        (return 0)))
    (else
      (return 0))))

(fn DetectPotentialTargets
  (params (Debug :type Boolean))
  (bind _capsulecomponent (Variables|Collision|GetCapsuleComponent))
  (bind (_outradius _outhalfheight) (Components|Capsule|GetScaledCapsuleSize _capsulecomponent))
  (Utilities|FlowControl|Sequence
    (:then_0
      (if Debug
        (Rendering|Debug|DrawDebugSphere (Transformation|GetActorLocation) (Variables|Default|GetMeleeAttackRange) 12 "(R=1.000000,G=0.000000,B=0.000000,A=1.000000)" 5.0)))
    (:then_1
      (bind _outactors (Collision|SphereOverlapActors (Transformation|GetActorLocation) (Variables|Default|GetMeleeAttackRange) (Variables|Default|GetTargetObjectTypes) 0 (Utilities|Array|MakeArray self)))
      (for _array_element _outactors
        (LocalVariables|SetLTestTarget _array_element)
        (Utilities|IsValid (Actor|GetComponentbyClass _array_element "/Game/MyContent/Core/BP_AC_Stats.BP_AC_Stats_C")
          (:Is%20Valid
            (if (Default|IsAlive (Actor|GetComponentbyClass _array_element "/Game/MyContent/Core/BP_AC_Stats.BP_AC_Stats_C"))
              (bind _returnvalue (Class|KismetSystemLibrary|CapsuleTraceSingleforObjects (Transformation|GetActorLocation) (Transformation|GetActorLocation (LocalVariables|GetLTestTarget)) (* _outradius 0.5) (* _outhalfheight 0.9) (Utilities|Array|MakeArray "ObjectTypeQuery1") false 0 (select Debug "ForDuration" "None") true))
              (if (not _returnvalue)
                (Utilities|Array|Add (LocalVariables|GetLPotentialTargets) (LocalVariables|GetLTestTarget)))))))
      (return (LocalVariables|GetLPotentialTargets) (Utilities|Array|IsNotEmpty (LocalVariables|GetLPotentialTargets))))))

(fn CompareTargetAngle
  (params (PotentialTargets :type Array%20of%20Actor%20Object%20References) (Debug :type Boolean))
  (for _array_element PotentialTargets
    (LocalVariables|SetLTestTarget _array_element)
    (if (>= (Math|Vector|DotProduct (Math|Vector|GetForwardVector (Math|Rotator|MakeRotator 0.0 0.0 (.yaw (Math|Rotator|FindLookatRotation (Transformation|GetActorLocation) (Transformation|GetActorLocation (LocalVariables|GetLTestTarget)))))) (Math|Vector|GetForwardVector (Math|Rotator|MakeRotator 0.0 0.0 (.yaw (Pawn|GetControlRotation :!class /Script/Engine.Pawn))))) (Variables|Default|GetSoftTargetAngle))
      ;[1 1 1] doesnt work
      (Utilities|Array|Add (LocalVariables|GetLTargetsWithAngle) (LocalVariables|GetLTestTarget))
      (if Debug
        (Rendering|Debug|DrawDebugBox (.Origin (Collision|GetActorBounds (LocalVariables|GetLTestTarget) true false)) (.BoxExtent (Collision|GetActorBounds (LocalVariables|GetLTestTarget) true false)) "(R=1.000000,G=0.733816,B=0.000000,A=1.000000)" (Transformation|GetActorRotation (LocalVariables|GetLTestTarget)) 5.0 0.0))))
  (return (LocalVariables|GetLTargetsWithAngle) (Utilities|Array|IsNotEmpty (LocalVariables|GetLTargetsWithAngle))))

(fn FindTargetClosesttoSelf
  (params (Actors :type Array%20of%20Actor%20Object%20References) (Debug :type Boolean))
  ;[1 1 1] doesnt work
  (for (_array_element _array_index) Actors
    (LocalVariables|SetLTestTarget _array_element)
    (if (or (== _array_index 0) (< (Class|KismetMathLibrary|VectorDistanceSquared (Transformation|GetActorLocation (LocalVariables|GetLTestTarget)) (CallFunction|GetLocationfromActorBasedonControl (Variables|Default|GetSoftTargetDistance))) 0.0))
      (LocalVariables|SetLClosestEntity (LocalVariables|GetLTestTarget))
      (LocalVariables|SetLClosestDistance (Class|KismetMathLibrary|VectorDistanceSquared (Transformation|GetActorLocation (LocalVariables|GetLTestTarget)) (CallFunction|GetLocationfromActorBasedonControl (Variables|Default|GetSoftTargetDistance))))))
  (Utilities|FlowControl|Sequence
    (:then_0
      (if Debug
        (Rendering|Debug|DrawDebugSphere (Transformation|GetActorLocation (LocalVariables|GetLClosestEntity)) 3e+01 12 "(R=0.154413,G=1.000000,B=0.000000,A=1.000000)" 5.0)
        ;[1 1 1] Doesnt work
        (Rendering|Debug|DrawDebugArrow :LineStart (Transformation|GetActorLocation) :LineEnd (CallFunction|GetLocationfromActorBasedonControl (Variables|Default|GetSoftTargetDistance)) :ArrowSize 5.0 :Duration 5.0)))
    (:then_1
      (return (LocalVariables|GetLClosestEntity)))))

(fn GetLocationfromActorBasedonControl
  (params (Distance :type Float%20%28double-precision%29))
  (return (+ (Transformation|GetActorLocation) (* (Math|Vector|GetForwardVector (Math|Rotator|MakeRotator 0.0 0.0 (.yaw (Pawn|GetControlRotation :!class /Script/Engine.Pawn)))) Distance))))

(fn SetWarpTarget
  (params (TargetActor :type Actor%20Object%20Reference))
  (Utilities|IsValid TargetActor
    (:Is%20Valid
      (Class|MotionWarpingComponent|AddorUpdateWarpTargetfromLocationandRotation (Variables|Default|GetMotionWarping) "BasicAttackTarget" (Transformation|GetActorLocation TargetActor) (Math|Rotator|FindLookatRotation (Transformation|GetActorLocation) (Transformation|GetActorLocation TargetActor))))
    (:Is%20Not%20Valid
      (Class|MotionWarpingComponent|RemoveWarpTarget (Variables|Default|GetMotionWarping) "BasicAttackTarget"))))

(fn PlayHitReact
  (Animation|Montage|MontagePlay (Components|SkeletalMesh|GetAnimInstance (Variables|Character|GetMesh)) "/Game/Sword_Animations/Animations/Sequence2/08_Hit/02_Hit_Combat/Player_Hit_Combat_F_Seq_Montage.Player_Hit_Combat_F_Seq_Montage" 1.0 "MontageLength" 0.0 true)
  (CallFunction|DeactivateWeaponDamage))